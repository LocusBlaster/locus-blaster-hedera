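; Bullet actor that kills AI enemies it touches and adds to the player's score.
; On spawn it plays a laser sound and destroys itself after a short lifetime.
; When its box begins an overlap, it checks every Ai_character for overlap, calls EnemyDeath on hits, increments Score on Bpc_character, then destroys itself after a brief delay.
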(event `self.ReceiveBeginPlay`
  (`GameplayStatics.PlaySoundAtLocation` "/Game/audio/effects/cue/laser_cue.laser_cue" (`self.K2_GetActorLocation`) (struct) 1.0 1.0 0.0 null null null null)
  (`KismetSystemLibrary.Delay` 1.0)
  (`self.K2_DestroyActor`))

(event `self.Box.OnComponentBeginOverlap`
  (params (OverlappedComponent :type "PrimitiveComponent Object Reference") (OtherActor :type "Actor Object Reference") (OtherComp :type "PrimitiveComponent Object Reference") (OtherBodyIndex :type Integer) (bFromSweep :type Boolean) (SweepResult :type "HitResult Structure (by ref)"))
  (bind _returnvalue (`GameplayStatics.GetActorOfClass` "/Game/player_character/blueprint/bpc_character.bpc_character_C"))
  (bind _outactors (`GameplayStatics.GetAllActorsOfClass` "/Game/ai_character/blueprint/ai_character.ai_character_C"))
  (for _array_element _outactors
    (if (`self.IsOverlappingActor` _array_element)
      (`/Game/ai_character/blueprint/ai_character.enemy_death` _array_element)
      (bind _result (`/Engine/EditorBlueprintResources/StandardMacros.IncrementInt` (`/Game/player_character/blueprint/bpc_character.score` _returnvalue))
        (:`  `
          (set `/Game/player_character/blueprint/bpc_character.score` _result _returnvalue)
          (`KismetSystemLibrary.Delay` 0.05)
          (`self.K2_DestroyActor`))))))

(fn `UserConstructionScript`)