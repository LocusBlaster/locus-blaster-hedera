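; Player character Blueprint for a flying space shooter: handles movement, firing, damage and game over.
; Enhanced Input drives horizontal and vertical movement and spawns bullets after a short delay.
; Box overlaps kill overlapping AI characters and damage the player, draining shield before health, which regenerates on a looping timer.
; Fatal damage pauses the game, shows the game-over widget and swaps the music.
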(event `self.ReceiveBeginPlay`
  (bind _returnvalue (`|CreateWidget` "/Game/widget/score_health.score_health_C"))
  (set `self.health_menu` _returnvalue)
  (`UserWidget.AddToViewport` (`self.health_menu`) 0)
  (bind _asplayer_controller (cast `PlayerController` (`self.GetController`)))
  (`EnhancedInputSubsystemInterface.AddMappingContext` (pcsubsystem `EnhancedInputLocalPlayerSubsystem` _asplayer_controller) "/Game/player_character/input/iac_input_context.iac_input_context" 0 (struct))
  (`CharacterMovementComponent.SetMovementMode` (`self.CharacterMovement`) "MOVE_Flying" 0)
  (`KismetSystemLibrary.K2_SetTimerDelegate` (delegate `regenerate`) 15.0 true)
  (`GameplayStatics.PlaySound2D` "/Game/audio/music/spaceEngine_003.spaceEngine_003" 1.0 1.0 0.0 null null)
  (bind _returnvalue_2 (`GameplayStatics.SpawnSound2D` "/Game/audio/music/game_song.game_song" 1.0 1.0 0.0 null))
  (set `self.game_sound_component` _returnvalue_2))

(event `EnhancedInput|/Game/player_character/input/ia_move_left_right`
  (params (ActionValue :type "Vector2D Structure") (ElapsedSeconds :type "Float (double-precision)") (TriggeredSeconds :type "Float (double-precision)") (InputAction :type "InputAction Object Reference" :default "/Game/player_character/input/ia_move_left_right.ia_move_left_right"))
  (:`Triggered`
    (`self.AddMovementInput` (`self.GetActorRightVector` (`self.GetController`)) ActionValue_X)))

(event `regenerate`
  (if (< (`self.health`) 1.0)
    (set `self.health` (+ (`self.health`) 0.2))))

(event `EnhancedInput|/Game/player_character/input/ia_move_up_down`
  (params (ActionValue :type "Vector2D Structure") (ElapsedSeconds :type "Float (double-precision)") (TriggeredSeconds :type "Float (double-precision)") (InputAction :type "InputAction Object Reference" :default "/Game/player_character/input/ia_move_up_down.ia_move_up_down"))
  (:`Triggered`
    (`self.AddMovementInput` (`self.GetActorUpVector` (`self.GetController`)) ActionValue_X)))

(event `EnhancedInput|/Game/player_character/input/ia_fire_weapon`
  (params (ActionValue :type Boolean) (ElapsedSeconds :type "Float (double-precision)") (TriggeredSeconds :type "Float (double-precision)") (InputAction :type "InputAction Object Reference" :default "/Game/player_character/input/ia_fire_weapon.ia_fire_weapon"))
  (:`Triggered`
    (`KismetSystemLibrary.Delay` 0.1)
    (`|SpawnActorFromClass` "/Game/other/bp_bullet.bp_bullet_C" (`self.GetTransform`) "AlwaysSpawn" "MultiplyWithRoot" null null)))

(event `take_damage`
  (bind _health (`self.health`))
  (bind _returnvalue (`|CreateWidget` "/Game/widget/damage.damage_C"))
  (`UserWidget.AddToViewport` _returnvalue 0)
  (if (> (`self.shield`) 0.2)
    (set `self.shield` (- (`self.shield`) 0.2))
    (elif (> _health 0.2)
      (set `self.health` (- _health 0.2))
      (else
        (`self.DisableInput` null)
        (bind _returnvalue_2 (`|CreateWidget` "/Game/widget/game_over_.game_over__C"))
        (set `PlayerController.bShowMouseCursor` true (`GameplayStatics.GetPlayerController` 0))
        (`UserWidget.AddToViewport` _returnvalue_2 0)
        (`AudioComponent.Stop` (`self.game_sound_component`))
        (`GameplayStatics.SetGamePaused` true)
        (bind _returnvalue_3 (`GameplayStatics.SpawnSound2D` "/Game/audio/music/loading_song.loading_song" 1.0 1.0 0.0 null))
        (set `self.game_over_component` _returnvalue_3)))))

(event `self.Box.OnComponentBeginOverlap`
  (params (OverlappedComponent :type "PrimitiveComponent Object Reference") (OtherActor :type "Actor Object Reference") (OtherComp :type "PrimitiveComponent Object Reference") (OtherBodyIndex :type Integer) (bFromSweep :type Boolean) (SweepResult :type "HitResult Structure (by ref)"))
  (bind _outactors (`GameplayStatics.GetAllActorsOfClass` "/Game/ai_character/blueprint/ai_character.ai_character_C"))
  (for _array_element _outactors
    (if (`self.IsOverlappingActor` _array_element)
      (`/Game/ai_character/blueprint/ai_character.enemy_death` _array_element)
      (`self.take_damage`))))

(fn `UserConstructionScript`)