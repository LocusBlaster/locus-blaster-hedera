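; Flying AI enemy character that moves along its controller's reversed forward vector, fires bullets and expires five seconds after spawning.
; Tick drives movement scaled by SpeedMultiplier and uses a random Delay as a fire timer, spawning Bp_enemy_bullet offset along world -X.
; Both timeout and enemy_death destroy the actor and then spawn an explosion effect; only enemy_death also plays the explosion sound.
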(event `self.ReceiveBeginPlay`
  (`CharacterMovementComponent.SetMovementMode` (`self.CharacterMovement`) "MOVE_Flying" 0)
  (`KismetSystemLibrary.Delay` 5.0)
  (`self.K2_DestroyActor`)
  (`self.spawn_explosion` :!label _label))

(event `self.ReceiveTick`
  (params (DeltaSeconds :type "Float (single-precision)"))
  (bind _returnvalue (`self.GetTransform`))
  (`self.AddMovementInput` (* (`self.GetActorForwardVector` (`self.GetController`)) DeltaSeconds (* (`self.Speed_multiplier`) -1)))
  (`KismetSystemLibrary.Delay` (`KismetMathLibrary.RandomFloatInRange` 0.1 1.0))
  (`|SpawnActorFromClass` "/Game/other/bp_enemy_bullet.bp_enemy_bullet_C" (`KismetMathLibrary.MakeTransform` (`KismetMathLibrary.MakeVector` (+ (.x (.location _returnvalue)) -500.0) (.y (.location _returnvalue)) (.z (.location _returnvalue))) (.rotation _returnvalue) (.scale _returnvalue)) "Undefined" "MultiplyWithRoot" null null))

(event `spawn_explosion`
  (bind (_returnvalue_location _returnvalue_rotation _returnvalue_scale) (`KismetMathLibrary.BreakTransform` (`self.GetTransform`)))
  (`GameplayStatics.SpawnEmitterAtLocation` "/Game/particles/Particles/P_Explosion.P_Explosion" _returnvalue_location _returnvalue_rotation _returnvalue_scale))

(event `enemy_death`
  (`GameplayStatics.PlaySoundAtLocation` "/Game/audio/effects/cue/explosion_cue.explosion_cue" (`self.K2_GetActorLocation`) (struct) 1.0 1.0 0.0 null null null null)
  (`self.K2_DestroyActor`)
  (goto _label))

(fn `UserConstructionScript`)