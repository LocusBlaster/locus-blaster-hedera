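; AI spawner actor that repeatedly spawns Ai_character enemies near the player.
; On BeginPlay it starts a looping timer whose interval is randomized once, then held for every repeat.
; Each spawn keeps the spawner's X, rotation and scale, randomizes Y and Z within ranges centered on the player's current position, and ignores collisions.
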(event `self.ReceiveBeginPlay`
  (`KismetSystemLibrary.K2_SetTimerDelegate` (delegate `spawn_enemy`) (`KismetMathLibrary.RandomFloatInRange` 0.5 5.0) true true))

(event `spawn_enemy`
  (bind _returnvalue (`self.GetTransform`))
  (bind _returnvalue_2 (`self.GetTransform` (`GameplayStatics.GetPlayerCharacter` 0)))
  (`|SpawnActorFromClass` "/Game/ai_character/blueprint/ai_character.ai_character_C" (`KismetMathLibrary.MakeTransform` (`KismetMathLibrary.MakeVector` (.x (.location _returnvalue)) (`KismetMathLibrary.RandomFloatInRange` (- (.y (.location _returnvalue_2)) 400.0) (+ (.y (.location _returnvalue_2)) 400.0)) (`KismetMathLibrary.RandomFloatInRange` (- (.z (.location _returnvalue_2)) 300.0) (+ (.z (.location _returnvalue_2)) 300.0))) (.rotation _returnvalue) (.scale _returnvalue)) "AlwaysSpawn" "MultiplyWithRoot" null null))

(fn `UserConstructionScript`)